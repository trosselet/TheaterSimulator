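; Main-level game mode for the cinema simulator that tracks connected players and supports kicking them.
; Login and logout add or remove each BP_MyPlayerController in an AllPlayerController array, then call UpdatePlayerList.
; An Update_PlayerList event waits briefly, then has BP_MyGameState refresh its player list.
; KickPlayer treats the given ID as an index into that array and calls OCKickPlayer on that controller.
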(event `Update_PlayerList`
  (`KismetSystemLibrary.Delay` 0.4)
  (bind _asbp_my_game_state (cast `/Game/CinemaSimulator/GameMode/MainLvl/BP_MyGameState` (`GameplayStatics.GetGameState`)))
  (`/Game/CinemaSimulator/GameMode/MainLvl/BP_MyGameState.Update_PlayerList` _asbp_my_game_state))

(event `self.K2_PostLogin`
  (params (NewPlayer :type "PlayerController Object Reference"))
  (bind _asbp_my_player_controller (cast `/Game/CinemaSimulator/GameMode/MainLvl/BP_MyPlayerController` NewPlayer))
  (`KismetArrayLibrary.Array_Add` (`self.All_PlayerController`) _asbp_my_player_controller)
  (`self.Update_PlayerList` :!label _label))

(event `self.K2_OnLogout`
  (params (ExitingController :type "Controller Object Reference"))
  (bind _asbp_my_player_controller (cast `/Game/CinemaSimulator/GameMode/MainLvl/BP_MyPlayerController` ExitingController))
  (`KismetArrayLibrary.Array_RemoveItem` (`self.All_PlayerController`) _asbp_my_player_controller)
  (goto _label))

(fn `KickPlayer`
  (params (PlayerId :type Integer))
  (`/Game/CinemaSimulator/GameMode/MainLvl/BP_MyPlayerController.OC_KickPlayer` (`|GetArrayItem` (`self.All_PlayerController`) PlayerId)))

(fn `UserConstructionScript`)