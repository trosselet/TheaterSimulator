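; BP_MainPlayer is the player pawn for the theater simulator, handling movement and horizontal turning through Enhanced Input.
; BeginPlay adds the IMC_Player mapping context, whose forward, right and turn actions drive movement input and controller yaw.
; Movement directions come from a rotator with control yaw wired into roll and yaw left at zero, so forward stays on world X regardless of facing.
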(event `self.ReceiveBeginPlay`
  (`EnhancedInputSubsystemInterface.AddMappingContext` (pcsubsystem `EnhancedInputLocalPlayerSubsystem` (`GameplayStatics.GetPlayerController` 0)) "/Game/TheaterSimulator/Input/IMC_Player.IMC_Player" 0 (struct)))

(event `EnhancedInput|/Game/TheaterSimulator/Input/IA_PlayerForward`
  (params (ActionValue :type "Float (double-precision)") (ElapsedSeconds :type "Float (double-precision)") (TriggeredSeconds :type "Float (double-precision)") (InputAction :type "InputAction Object Reference" :default "/Game/TheaterSimulator/Input/IA_PlayerForward.IA_PlayerForward"))
  (:`Triggered`
    (`self.AddMovementInput` (`KismetMathLibrary.GetForwardVector` (`KismetMathLibrary.MakeRotator` (.yaw (`Controller.GetControlRotation` (`GameplayStatics.GetPlayerController` 0))))) ActionValue)))

(event `EnhancedInput|/Game/TheaterSimulator/Input/IA_PlayerRight`
  (params (ActionValue :type "Float (double-precision)") (ElapsedSeconds :type "Float (double-precision)") (TriggeredSeconds :type "Float (double-precision)") (InputAction :type "InputAction Object Reference" :default "/Game/TheaterSimulator/Input/IA_PlayerRight.IA_PlayerRight"))
  (:`Triggered`
    (`self.AddMovementInput` (`KismetMathLibrary.GetRightVector` (`KismetMathLibrary.MakeRotator` (.yaw (`Controller.GetControlRotation` (`GameplayStatics.GetPlayerController` 0))))) ActionValue)))

(event `EnhancedInput|/Game/TheaterSimulator/Input/IA_PlayerTurn`
  (params (ActionValue :type "Float (double-precision)") (ElapsedSeconds :type "Float (double-precision)") (TriggeredSeconds :type "Float (double-precision)") (InputAction :type "InputAction Object Reference" :default "/Game/TheaterSimulator/Input/IA_PlayerTurn.IA_PlayerTurn"))
  (:`Triggered`
    (`self.AddControllerYawInput` ActionValue)))

(fn `UserConstructionScript`)