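; BP_MyPlayerController is the player controller in the CinemaSimulator main-level game mode folder, handling the player list and being kicked from a session.
; BeginPlay adds a WBP_PlayerList widget to the viewport, focuses it in Game and UI input mode and shows the cursor.
; Holding Tab shows the list and cursor, and releasing hides both.
; OC_KickPlayer opens the main menu level, then destroys the session.
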(event `self.ReceiveBeginPlay`
  (bind _returnvalue (`|CreateWidget` "/Game/CinemaSimulator/Levels/MainMap/UI/WBP_PlayerList.WBP_PlayerList_C" self))
  (`UserWidget.AddToViewport` _returnvalue 0)
  (`WidgetBlueprintLibrary.SetInputMode_GameAndUIEx` self _returnvalue :!label _label)
  (set `self.bShowMouseCursor` true))

(event `Key|Tab`
  (params (Key :type "Key Structure"))
  (:`Pressed`
    (`Widget.SetVisibility` (stale `self.ReceiveBeginPlay` _returnvalue) "Visible")
    (goto _label))
  (:`Released`
    (`Widget.SetVisibility` (stale `self.ReceiveBeginPlay` _returnvalue) "Hidden")
    (`WidgetBlueprintLibrary.SetInputMode_GameAndUIEx` self (stale `self.ReceiveBeginPlay` _returnvalue))
    (set `self.bShowMouseCursor` false)))

(event `OC_KickPlayer`
  (`GameplayStatics.OpenLevelBySoftObjectPtr` "/Game/CinemaSimulator/Levels/MainMenu/LV_MainMenu.LV_MainMenu")
  (`DestroySessionCallbackProxy.DestroySession` null
    (:`OnSuccess`
      (`KismetSystemLibrary.PrintString` "Got Kicked"))))

(fn `UserConstructionScript`)